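; MoveObstacleDown is an obstacle actor that travels vertically, reversing between up and down about every five seconds.
; Each Tick moves it without sweep along the normalized Vector variable, scaled by delta seconds and the Float speed variable.
; The same Tick feeds a Delay, which ignores retriggers while pending, so its FlipFlop acts as a repeating timer that alternates Vector between upward and downward.
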(event `self.ReceiveTick`
  (params (DeltaSeconds :type "Float (single-precision)"))
  (`self.K2_SetActorLocation` (+ (* (`KismetMathLibrary.Normal` (`self.Vector`)) (* (`GameplayStatics.GetWorldDeltaSeconds`) (`self.float`))) (.location (`SceneComponent.K2_GetComponentToWorld` (`self.DefaultSceneRoot`)))))
  (`KismetSystemLibrary.Delay` 5.0)
  (`/Engine/EditorBlueprintResources/StandardMacros.FlipFlop`
    (:`A`
      (set `self.Vector` (0.0 0.0 30.0)))
    (:`B`
      (set `self.Vector` (0.0 0.0 -30.0)))))

(fn `UserConstructionScript`)