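; MoveObstacle is an obstacle actor that shuttles along alternating directions at a constant speed.
; Each Tick offsets the root's world location along the normalized Vector, scaled by Float and delta time, without sweeping for collision.
; A Delay on Tick serves as a repeating timer, feeding a FlipFlop that switches Vector between Vectottran and Vectottran0.
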(event `self.ReceiveTick`
  (params (DeltaSeconds :type "Float (single-precision)"))
  (`self.K2_SetActorLocation` (+ (* (`KismetMathLibrary.Normal` (`self.Vector`)) (* (`GameplayStatics.GetWorldDeltaSeconds`) (`self.float`))) (.location (`SceneComponent.K2_GetComponentToWorld` (`self.DefaultSceneRoot`)))))
  (`KismetSystemLibrary.Delay` (`self.delay`))
  (`/Engine/EditorBlueprintResources/StandardMacros.FlipFlop`
    (:`A`
      (set `self.Vector` (`self.Vectottran`)))
    (:`B`
      (set `self.Vector` (`self.Vectottran_0`)))))

(fn `UserConstructionScript`)