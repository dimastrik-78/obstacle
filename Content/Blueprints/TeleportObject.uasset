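; Actor Blueprint that teleports itself back and forth 500 units along the world X axis at timed intervals.
; Tick feeds a Delay, then a FlipFlop alternates between adding and subtracting the offset with an unswept location set.
; The first jump waits Delta, which is then overwritten by DeltaAfterTp; the return branch assigns Delta to itself, so the original interval is never restored.
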(event `self.ReceiveTick`
  (params (DeltaSeconds :type "Float (single-precision)"))
  (bind _delta (`self.delta`))
  (bind _location (.location (`self.GetTransform`)))
  (`KismetSystemLibrary.Delay` _delta)
  (`/Engine/EditorBlueprintResources/StandardMacros.FlipFlop`
    (:`A`
      (`self.K2_SetActorLocation` (+ _location (500.0 0.0 0.0)))
      (set `self.delta` (`self.delta_after_tp`)))
    (:`B`
      (`self.K2_SetActorLocation` (- _location (500.0 0.0 0.0)))
      (set `self.delta` _delta))))

(fn `UserConstructionScript`)